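; Launch pad button that plays a press animation and sound, and reports whether the launch pad is active.
; ButtonPressed runs chained timelines that lerp the mesh between cached normal and offset transforms, then prints a status from IsTheButtonPressed, which is not set here.
; Collision enter and leave events add and remove an interact prompt widget, whose key-pressed state flashes briefly on Interact input.
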(event EventBeginPlay
  (bind _buttonmeshcomponent (Variables|Default|GetButtonMeshComponent))
  (bind _returnvalue (Transformation|GetRelativeTransform _buttonmeshcomponent))
  (Variables|Default|SetNormal%20Button%20Position (Math|Transform|MakeTransform (.location _returnvalue) (.rotation _returnvalue) (.scale _returnvalue)))
  (Variables|Default|SetPressed%20Button%20Position (Math|Transform|MakeTransform (- (.location _returnvalue) "0, 0,-10.000000") (.rotation _returnvalue) (.scale _returnvalue))))

(event Collision|EventActorBeginOverlap
  (params (OtherActor :type Actor%20Object%20Reference)))

(event EventTick
  (params (DeltaSeconds :type Float%20%28single-precision%29)))

(event EventButtonPressed
  (Utilities|FlowControl|Sequence
    (:then_0
      (Audio|PlaySoundatLocation "/Game/SoundEffects/ButtonSoundEffect.ButtonSoundEffect" (Transformation|GetActorLocation) "0, 0, 0" 1.0 1.0 0.0 0 0 0)
      ;[1 1 1] Move Button in Animation
      (bind _button_in (Timeline|Button_In PlayFromStart)
        (:Update
          (Transformation|SetRelativeTransform (Variables|Default|GetButtonMeshComponent) (Math|Transform|Lerp(Transform) (Variables|Default|GetNormal%20Button%20Position) (Variables|Default|GetPressed%20Button%20Position) _button_in) false false))
        (:Finished
          ;[1 1 1] Move Button Out Animation
          (bind _button_in_2 (Timeline|Button_Out ReverseFromEnd)
            (:Update
              (Transformation|SetRelativeTransform (Variables|Default|GetButtonMeshComponent) (Math|Transform|Lerp(Transform) (Variables|Default|GetNormal%20Button%20Position) (Variables|Default|GetPressed%20Button%20Position) _button_in_2) false false))))))
    (:then_1
      (if (Variables|Default|GetbIsTheButtonPressed)
        (Development|PrintString "LaunchPad is now Active" true true "(R=0.000000,G=0.812500,B=0.039431,A=1.000000)")
        (else
          (Development|PrintString "LaunchPad is now Inactive" true true "(R=1.000000,G=0.034517,B=0.074318,A=1.000000)"))))))

(event EventCharacterEntersCollision
  ;[1 1 1] Check Player Proximity
  ;[1 1 1] Show Interact Icon
  (bind _returnvalue (UserInterface|CreateWidget "/Game/UI/WBP_PressKeyToInteract.WBP_PressKeyToInteract_C"))
  (UserInterface|Viewport|AddtoViewport _returnvalue 0))

(event EventCharacterLeavesCollision
  ;[1 1 1] Check Player Proximity
  ;[1 1 1] Show Interact Icon
  (Widget|RemovefromParent (stale EventCharacterEntersCollision _returnvalue)))

(event Input|ActionEvents|InputActionInteract
  (params (Key :type Key%20Structure))
  ;[1 1 1] Change the widget
  (:Pressed
    (Variables|/Game/UI/WBP_PressKeyToInteract.WBP_PressKeyToInteract_C|SetbIsKeyPressed (stale EventCharacterEntersCollision _returnvalue) true)
    (Utilities|FlowControl|Delay 0.2)
    (Variables|/Game/UI/WBP_PressKeyToInteract.WBP_PressKeyToInteract_C|SetbIsKeyPressed (stale EventCharacterEntersCollision _returnvalue) false)))

(fn ConstructionScript)