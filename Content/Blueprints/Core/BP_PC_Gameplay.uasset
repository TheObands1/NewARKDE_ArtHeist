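; Gameplay player controller that shows and hides the pause menu and switches input modes to match.
; PauseGame creates the W_PauseMenu widget on first use, reuses the cached reference afterwards, and enables UI-only input with a visible cursor.
; UnPauseGame removes the widget and restores game-only input, which is also set at BeginPlay, and hides the cursor.
; Neither event changes the game's actual paused state.
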(event EventBeginPlay
  (Input|SetInputModeGameOnly self))

(event EventTick
  (params (DeltaSeconds :type Float%20%28single-precision%29)))

(event EventPauseGame
  (params (NewState :type Boolean))
  (bind _returnvalue (Game|GetPlayerController 0))
  (Utilities|IsValid (Variables|Default|GetW_PauseMenuReference)
    (:Is%20Valid
      _)
    (:Is%20Not%20Valid
      (bind _returnvalue_2 (UserInterface|CreateWidget "/Game/UI/PauseMenu/W_PauseMenu.W_PauseMenu_C"))
      (bind _output_get (Variables|Default|SetW_PauseMenuReference _returnvalue_2))))
  (UserInterface|Viewport|AddtoViewport _output_get 0)
  (Input|SetInputModeUIOnly _returnvalue 0 "DoNotLock")
  (Variables|/Script/Engine.PlayerController|SetbShowMouseCursor _returnvalue true))

(event EventUnPauseGame
  (params (NewState :type Boolean))
  (bind _returnvalue (Game|GetPlayerController 0))
  (bind _w_pausemenureference (Variables|Default|GetW_PauseMenuReference))
  (Utilities|IsValid _w_pausemenureference
    (:Is%20Valid
      (Widget|RemovefromParent _w_pausemenureference)
      (Input|SetInputModeGameOnly _returnvalue)
      (Variables|/Script/Engine.PlayerController|SetbShowMouseCursor _returnvalue false))))

(fn ConstructionScript)