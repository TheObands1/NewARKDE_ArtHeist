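; AIC_Enemy is the enemy AI controller Blueprint with an AI Perception component, but none of its live events do any work.
; Two disconnected chains preserve a Blueprint version of the setup, labelled as the "Blueprint way".
; One would run BT_Enemy and copy patrol settings from the AH_Enemy pawn to the Blackboard.
; The other would turn player sight and damage stimuli, told apart by array index, into Blackboard chase and investigation keys.
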(event OnPerceptionUpdated(AIPerception)
  (params (UpdatedActors :type Array%20of%20Actor%20Object%20References)))

(event EventBeginPlay)

(event EventTick
  (params (DeltaSeconds :type Float%20%28single-precision%29)))

(fn ConstructionScript)