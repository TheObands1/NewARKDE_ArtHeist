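; BP_Door is a door that swings open and can report that the player needs a key.
; OpenDoor plays a timeline that lerps the DoorComponent's yaw from its current value toward OpenAngle, re-reading that yaw on every update.
; PlayerNeedsKey prints an on-screen message naming the required key from DoorTag.
; The key check and calls to both events are not in these graphs.
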(event EventBeginPlay)

(event Collision|EventActorBeginOverlap
  (params (OtherActor :type Actor%20Object%20Reference)))

(event EventTick
  (params (DeltaSeconds :type Float%20%28single-precision%29)))

(event EventOpenDoor
  (bind _openstate (Timeline|TL_OpenDoor PlayFromStart)
    (:Update
      (Transformation|SetRelativeRotation (Variables|Default|GetDoorComponent) (Math|Rotator|MakeRotator 0.0 0.0 (Math|Float|Lerp (.Yaw (Math|Rotator|BreakRotator (Variables|/Script/Engine.SceneComponent|GetRelativeRotation (Variables|Default|GetDoorComponent)))) (Variables|Default|GetOpenAngle) _openstate)) false false))))

(event EventPlayerNeedsKey
  (Development|PrintString (Utilities|String|Append "You need this key to enter: " (Utilities|String|ToString(Name) (Variables|Default|GetDoorTag))) true true "(R=1.000000,G=0.032523,B=0.000000,A=1.000000)" 3.0))

(fn ConstructionScript)