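; BP_LaunchPad is a launch pad actor that briefly displays a sign showing whether it is active.
; Both the activation and deactivation sign components are hidden on BeginPlay.
; The ShowActivationStatusSign event checks IsLaunchPadActive, shows the matching sign while hiding the other, then hides it after a five-second delay.
; The launch behavior itself is not in this graph.
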(event EventBeginPlay
  (Rendering|SetVisibility (Variables|Default|GetActivationSignComponent) false false)
  (Rendering|SetVisibility (Variables|Default|GetDeActivationSignComponent) false false))

(event Collision|EventActorBeginOverlap
  (params (OtherActor :type Actor%20Object%20Reference)))

(event EventTick
  (params (DeltaSeconds :type Float%20%28single-precision%29)))

(event EventShowActivationStatusSign
  (if (Variables|Default|GetbIsLaunchPadActive)
    (Rendering|SetVisibility (Variables|Default|GetDeActivationSignComponent) false false)
    (Rendering|SetVisibility (Variables|Default|GetActivationSignComponent) true false)
    (Utilities|FlowControl|Delay 5.0)
    (Rendering|SetVisibility (Variables|Default|GetActivationSignComponent) false false)
    (else
      (Rendering|SetVisibility (Variables|Default|GetActivationSignComponent) false false)
      (Rendering|SetVisibility (Variables|Default|GetDeActivationSignComponent) true false)
      (Utilities|FlowControl|Delay 5.0)
      (Rendering|SetVisibility (Variables|Default|GetDeActivationSignComponent) false false))))

(fn ConstructionScript)