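; Player character Blueprint that adds HUD, camera selection and visual feedback for rifle and melee ultimates.
; BeginPlay creates the main HUD and caches post-process settings, which ultimates swap for a type-specific tint and restore on stop.
; During a melee ultimate, two detector components spawn distinct Niagara claw and slash effects on overlapped enemies.
; The construction script auto-activates either the first-person or spring-arm third-person camera, and landing resets the jump counter.
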(event OnComponentBeginOverlap(MeleeDetectorComponent)
  (params (OverlappedComponent :type Primitive%20Component%20Object%20Reference) (OtherActor :type Actor%20Object%20Reference) (OtherComp :type Primitive%20Component%20Object%20Reference) (OtherBodyIndex :type Integer) (bFromSweep :type Boolean) (SweepResult :type Hit%20Result%20Structure%20%28by%20ref%29))
  (if (Variables|Default|GetbIsUsingUltimate)
    (if (Utilities|Enum|Equal(Enum) (Variables|Default|GetCurrentUltimateType) "UltimateType_Melee")
      (Utilities|Casting|CastToBP_Enemy OtherActor)
      (Niagara|SpawnSystematLocation "/Game/Game_Assets/Hack_And_Slash_FX/VFX_Niagara/Demo_Together/NS_Claws_Floor_NS_Claws_Together.NS_Claws_Floor_NS_Claws_Together" (Transformation|GetActorLocation OtherActor) (Transformation|GetSocketRotation (Variables|Default|GetMeleeDetectorComponent) "None") "1.500000,1.500000,1.500000"))))

(event OnComponentBeginOverlap(MeleeArmDetectorComponent)
  (params (OverlappedComponent :type Primitive%20Component%20Object%20Reference) (OtherActor :type Actor%20Object%20Reference) (OtherComp :type Primitive%20Component%20Object%20Reference) (OtherBodyIndex :type Integer) (bFromSweep :type Boolean) (SweepResult :type Hit%20Result%20Structure%20%28by%20ref%29))
  (if (Variables|Default|GetbIsUsingUltimate)
    (if (Utilities|Enum|Equal(Enum) (Variables|Default|GetCurrentUltimateType) "UltimateType_Melee")
      (Utilities|Casting|CastToBP_Enemy OtherActor)
      (Niagara|SpawnSystematLocation "/Game/Game_Assets/Hack_And_Slash_FX/VFX_Niagara/Demo_Together/NS_Demon_Slash_Together.NS_Demon_Slash_Together" (Transformation|GetActorLocation OtherActor) (Transformation|GetSocketRotation (Variables|Default|GetMeleeArmDetectorComponent) "None") "1.500000,1.500000,1.500000"))))

(event EventBeginPlay
  (Utilities|FlowControl|Sequence
    (:then_0
      (bind _returnvalue (UserInterface|CreateWidget "/Game/UI/HUD/W_MainHUD.W_MainHUD_C"))
      (UserInterface|Viewport|AddtoViewport _returnvalue 0))
    (:then_1
      (Variables|Default|SetNormalSettings (Variables|/Script/Engine.PostProcessComponent|GetSettings (Variables|Default|GetPostProcess))))))

(event Collision|EventActorBeginOverlap
  (params (OtherActor :type Actor%20Object%20Reference)))

(event EventTick
  (params (DeltaSeconds :type Float%20%28single-precision%29)))

(event EventOnLanded
  (params (Hit :type Hit%20Result%20Structure%20%28by%20ref%29))
  (Variables|Default|SetJumpCounter 0))

(event EventStartUltimate
  (params (UltimateType :type EAH_UltimateType%20Enum :default "UltimateType_Rifle"))
  (if (Utilities|Enum|Equal(Enum) UltimateType "UltimateType_Rifle")
    (Variables|/Script/Engine.PostProcessComponent|SetSettings (Variables|Default|GetPostProcess) (Utilities|Struct|MakePostProcessSettings 1.0 0.0 0.7))
    (elif (Utilities|Enum|Equal(Enum) UltimateType "UltimateType_Melee")
      (Variables|/Script/Engine.PostProcessComponent|SetSettings (Variables|Default|GetPostProcess) (Utilities|Struct|MakePostProcessSettings -1.0 0.0 0.7)))))

(event EventStopUltimate
  (params (UltimateType :type EAH_UltimateType%20Enum :default "UltimateType_Rifle"))
  (Variables|/Script/Engine.PostProcessComponent|SetSettings (Variables|Default|GetPostProcess) (Variables|Default|GetNormalSettings)))

(fn ConstructionScript
  (Components|Activation|SetAutoActivate (Variables|Default|GetFPSCameraComponent) (Variables|Default|GetbUseFirstPersonView))
  (Components|Activation|SetAutoActivate (Variables|Default|GetTPSCameraComponent) (not (Variables|Default|GetbUseFirstPersonView))))